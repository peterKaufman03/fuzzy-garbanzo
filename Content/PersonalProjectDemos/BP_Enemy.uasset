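; BP_Enemy is a simple demo enemy that greets the player with a threat and can be killed by damage.
; BeginPlay prints a taunt to the screen.
; A TakeDamage event prints a pain message, subtracts the amount from Health, and destroys the actor when the CheckIfDead helper finds Health at or below zero.
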(event `self.ReceiveBeginPlay`
  (`KismetSystemLibrary.PrintString` "Hello, I have been programmed to destroy you!"))

(event `Take Damage`
  (params (`By Amount` :type "Float (double-precision)" :default 0.2))
  (`KismetSystemLibrary.PrintString` "Ouuuuuchhh")
  (set `self.Health` (- (`self.Health`) `By Amount`))
  (if (`self.CheckIfDead` (`self.Health`))
    (`self.K2_DestroyActor`)))

(fn `CheckIfDead`
  (params (Health :type "Float (double-precision)"))
  (returns (IsDead :type Boolean))
  (return (<= Health 0.0)))

(fn `UserConstructionScript`)