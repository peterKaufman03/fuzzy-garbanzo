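; BP_EnemyTester is a test Blueprint that repeatedly damages every BP_Enemy in the level.
; From BeginPlay, it gathers all enemies, prints their count, calls TakeDamage on each with a small random amount, then prints a confirmation.
; After a short delay, the GiveDamage custom event re-enters the same chain, so the search and damage pass repeats indefinitely.
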(event `self.ReceiveBeginPlay`
  (bind _outactors (`GameplayStatics.GetAllActorsOfClass` "/Game/PersonalProjectDemos/BP_Enemy.BP_Enemy_C" :!label _label)) ; finds all BP enemies
  (`KismetSystemLibrary.PrintString` (`KismetStringLibrary.Concat_StrStr` "There are " (`KismetStringLibrary.Conv_IntToString` (`KismetArrayLibrary.Array_Length` _outactors)) " in the level") true true (struct :`G` 0.66 :`B` 1.0 :`A` 1.0) 5.0)
  (for _array_element _outactors
    (`/Game/PersonalProjectDemos/BP_Enemy.Take Damage` _array_element (`KismetMathLibrary.RandomFloatInRange` 0.1 0.5)))
  (`KismetSystemLibrary.PrintString` "Gave Damage to all Enemies.")
  (`KismetSystemLibrary.Delay` 2.0) ; Damage Loop
  (`self.Give Damage`))

(event `Give Damage`
  (goto _label))

(fn `UserConstructionScript`)