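; BP_Item is an item Blueprint with pick-up, drop and primary-action events.
; PickUp disables the Cube's collision and attaches to the supplied parent's right item socket, snapping location and rotation.
; Drop detaches the Cube in world space, restores collision, enables physics and applies a mostly upward acceleration to toss it.
; PrimaryAction is a placeholder that only prints a debug message, as the other events also do.
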(event `PickUp`
  (params (`Mesh Component` :type "SceneComponent Object Reference") (Parent :type "SceneComponent Object Reference"))
  (`KismetSystemLibrary.PrintString` "Call Pickup" true true (struct :`R` 1.0 :`G` 0.247524 :`B` 0.369464 :`A` 1.0))
  (`PrimitiveComponent.SetCollisionEnabled` (`self.Cube`) "NoCollision")
  (`self.K2_AttachToComponent` Parent "item_socket_r" "SnapToTarget" "SnapToTarget" "KeepRelative"))

(event `Drop`
  (`KismetSystemLibrary.PrintString` "Call Drop" true true (struct :`R` 1.0 :`G` 0.238722 :`B` 0.198916 :`A` 1.0))
  (`SceneComponent.K2_DetachFromComponent` (`self.Cube`) "KeepWorld" "KeepWorld" "KeepWorld" true)
  (`PrimitiveComponent.SetCollisionEnabled` (`self.Cube`) "QueryAndPhysics")
  (`PrimitiveComponent.SetSimulatePhysics` (`self.Cube`) true)
  (`PrimitiveComponent.AddForce` (`self.Cube`) (10.0 0.0 5000.0) "None" true))

(event `PrimaryAction`
  (`KismetSystemLibrary.PrintString` "Call PrimaryAction" true true (struct :`R` 1.0 :`G` 0.208026 :`B` 0.319841 :`A` 1.0)))

(fn `UserConstructionScript`)