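; BP_Launcher is a revolver-mesh launcher that fires BP_Projectile actors on its PrimaryAction event.
; Firing prints a debug message, disables collision on the revolver mesh and Cube, then spawns a projectile at the Cube's transform.
; It enables physics on the projectile's Sphere, but applies the forward acceleration force to the launcher's own Cube rather than the projectile.
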(event `self.PrimaryAction`
  (bind (_returnvalue_location _returnvalue_rotation _returnvalue_scale) (`KismetMathLibrary.BreakTransform` (`SceneComponent.K2_GetComponentToWorld` (`self.Cube`))))
  (if true
    (`KismetSystemLibrary.PrintString` "Blam!")
    (`PrimitiveComponent.SetCollisionEnabled` (`self.SM_Wep_Revolver_01_Preset_01`) "NoCollision")
    (`PrimitiveComponent.SetCollisionEnabled` (`self.Cube`) "NoCollision")
    (bind _returnvalue (`|SpawnActorFromClass` "/Game/PersonalProjectDemos/BP_Projectile.BP_Projectile_C" (`KismetMathLibrary.MakeTransform` (+ _returnvalue_location (0.0 0.0 0.0)) _returnvalue_rotation _returnvalue_scale) "Undefined" "MultiplyWithRoot" null null)) ; Spawn the bullet above the player's head
    (`PrimitiveComponent.SetSimulatePhysics` (`/Game/PersonalProjectDemos/BP_Projectile.Sphere` _returnvalue) true)
    (`PrimitiveComponent.AddForce` (`self.Cube`) (* (`SceneComponent.GetForwardVector` (`self.Cube`)) 250000.0) "None" true) ; Shoot the bullet in the camera's direction
  ))

(fn `UserConstructionScript`
  (`parent.UserConstructionScript`))