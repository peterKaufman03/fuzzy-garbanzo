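; BP_BaronsThroneandPrince_Book is an interactable book that shows the W_BaronsBook widget when its PrimaryAction event fires.
; The event disables collision on the Cube, adds the widget to the viewport, then removes all top-level widgets of that class after a fixed delay.
; A closing branch also exists, but the condition is hardwired to true, so it never runs.
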(event `self.PrimaryAction`
  (if true
    (`KismetSystemLibrary.PrintString` "The book is open.")
    (`PrimitiveComponent.SetCollisionEnabled` (`self.Cube`) "NoCollision")
    (bind _returnvalue (`|CreateWidget` "/Game/ToonGame/UI/W_BaronsBook.W_BaronsBook_C"))
    (`UserWidget.AddToViewport` _returnvalue 0)
    (`KismetSystemLibrary.Delay` 15.0)
    (bind _foundwidgets (`WidgetBlueprintLibrary.GetAllWidgetsOfClass` "/Game/ToonGame/UI/W_BaronsBook.W_BaronsBook_C"))
    (`Widget.RemoveFromParent` _foundwidgets)
    (else
      (`KismetSystemLibrary.PrintString` "The book is closed.")
      (`PrimitiveComponent.SetCollisionEnabled` (`self.Cube`) "NoCollision")
      (`WidgetLayoutLibrary.GetViewportWidgetGeometry`)
      (bind _foundwidgets_2 (`WidgetBlueprintLibrary.GetAllWidgetsOfClass` "/Game/ToonGame/UI/W_BaronsBook.W_BaronsBook_C"))
      (`Widget.RemoveFromParent` _foundwidgets_2))))

(fn `UserConstructionScript`
  (`parent.UserConstructionScript`))