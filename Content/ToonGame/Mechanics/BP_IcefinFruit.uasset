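; BP_IcefinFruit is an item Blueprint that plays a timed text sequence when its PrimaryAction fires.
; It creates a WP_ItemText widget and steps through the IcefinFruitText array by StoryIndex, showing each line for four seconds via a looped Delay.
; After the last line, it removes all top-level WP_ItemText widgets from the screen; StoryIndex is never reset here.
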(event `self.PrimaryAction`
  (bind _returnvalue (`|CreateWidget` "/Game/ToonGame/Mechanics/WP_ItemText.WP_ItemText_C"))
  (`UserWidget.AddToViewport` _returnvalue 0)
  (set `/Game/ToonGame/Mechanics/WP_ItemText.Item Text` (`|GetArrayItem` (`self.IcefinFruitText`) (`self.StoryIndex`)) _returnvalue :!label _label)
  (`KismetSystemLibrary.Delay` 4.0)
  (`/Engine/EditorBlueprintResources/StandardMacros.IncrementInt` (`self.StoryIndex`)
    (:`  `
      (if (< (`self.StoryIndex`) (`KismetArrayLibrary.Array_Length` (`self.IcefinFruitText`)))
        (goto _label)
        (else
          (bind _foundwidgets (`WidgetBlueprintLibrary.GetAllWidgetsOfClass` "/Game/ToonGame/Mechanics/WP_ItemText.WP_ItemText_C"))
          (`Widget.RemoveFromParent` _foundwidgets))))))

(fn `UserConstructionScript`
  (`parent.UserConstructionScript`))