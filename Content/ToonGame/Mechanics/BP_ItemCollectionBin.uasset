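; BP_ItemCollectionBin is a collection bin that counts items placed in it.
; When a BP_Item begins overlapping its ItemCollection component, it decrements ItemsLeft on BP_ThirdPersonGameMode and prints the remaining count.
; End overlap only casts to BP_Item, so leaving the bin never restores the count.
; Disconnected nodes hold an unfinished all-items-collected check and a tag-based round lookup, neither of which runs.
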(event `self.ItemCollection.OnComponentBeginOverlap`
  (params (OverlappedComponent :type "PrimitiveComponent Object Reference") (OtherActor :type "Actor Object Reference") (OtherComp :type "PrimitiveComponent Object Reference") (OtherBodyIndex :type Integer) (bFromSweep :type Boolean) (SweepResult :type "HitResult Structure (by ref)"))
  (cast `/Game/ToonGame/Mechanics/BP_Item` OtherActor)
  (bind _asbp_third_person_game_mode (cast `/Game/ThirdPerson/Blueprints/BP_ThirdPersonGameMode` (`GameplayStatics.GetGameMode`)))
  (bind _result (`/Engine/EditorBlueprintResources/StandardMacros.DecrementInt` (`/Game/ThirdPerson/Blueprints/BP_ThirdPersonGameMode.ItemsLeft` _asbp_third_person_game_mode))
    (:`  `
      (bind _output_get (set `/Game/ThirdPerson/Blueprints/BP_ThirdPersonGameMode.ItemsLeft` _result _asbp_third_person_game_mode))
      (`KismetSystemLibrary.PrintString` (`KismetStringLibrary.Conv_IntToString` _output_get)))))

(event `self.ItemCollection.OnComponentEndOverlap`
  (params (OverlappedComponent :type "PrimitiveComponent Object Reference") (OtherActor :type "Actor Object Reference") (OtherComp :type "PrimitiveComponent Object Reference") (OtherBodyIndex :type Integer))
  (cast `/Game/ToonGame/Mechanics/BP_Item` OtherActor))

(fn `UserConstructionScript`)