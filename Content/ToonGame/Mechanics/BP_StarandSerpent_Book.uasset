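; BP_StarandSerpent_Book is an interactable book prop that shows an open-book UI when it receives PrimaryAction.
; The action disables collision on the Cube and SMPropBook01 components, adds a W_OpenBook widget to the viewport, and removes all widgets after an eight-second delay.
; Its branch condition is hard-coded true, so the book-closed path never runs.
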(event `self.PrimaryAction`
  (if true
    (`KismetSystemLibrary.PrintString` "The book is open.")
    (`PrimitiveComponent.SetCollisionEnabled` (`self.Cube`) "NoCollision")
    (`PrimitiveComponent.SetCollisionEnabled` (`self.SM_Prop_Book_01`) "NoCollision")
    (bind _returnvalue (`|CreateWidget` "/Game/ToonGame/UI/W_OpenBook.W_OpenBook_C"))
    (`UserWidget.AddToViewport` _returnvalue 0)
    (`KismetSystemLibrary.Delay` 8.0)
    (`WidgetLayoutLibrary.RemoveAllWidgets`)
    (else
      (`KismetSystemLibrary.PrintString` "The book is closed.")
      (`PrimitiveComponent.SetCollisionEnabled` (`self.Cube`) "NoCollision")
      (`PrimitiveComponent.SetCollisionEnabled` (`self.SM_Prop_Book_01`) "NoCollision")
      (`WidgetLayoutLibrary.GetViewportWidgetGeometry`)
      (`WidgetLayoutLibrary.RemoveAllWidgets`))))

(fn `UserConstructionScript`
  (`parent.UserConstructionScript`))